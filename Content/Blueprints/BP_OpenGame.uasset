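; BP_OpenGame is a Mixed Reality UX Tools panel actor with a close button and optional experimental-warning text.
; The Construction Script sets warning title and body visibility from ShowExperimentalWarning.
; BeginPlay binds the CloseButton child actor's release event to Close, which hides the BP_OpenGame actor found by class lookup.
; The ShowHelp visibility-swap handler is bound only in disconnected setup logic, and CloseParent is empty.
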(event Custom|Close
  (params (Button :type Uxt%20Pressable%20Button%20Component%20Object%20Reference) (Pointer :type Uxt%20Pointer%20Component%20Object%20Reference))
  (bind _returnvalue (Actor|GetActorOfClass "BP_OpenGame_C"))
  (Rendering|SetActorHiddenInGame _returnvalue true))

(event Custom|ShowHelp
  (params (Button :type Uxt%20Pressable%20Button%20Component%20Object%20Reference) (Pointer :type Uxt%20Pointer%20Component%20Object%20Reference))
  (Utilities|FlowControl|Sequence
    (:then_0
      (bind _returnvalue (Actor|GetActorOfClass "BP_OpenGame_C"))
      (Rendering|SetActorHiddenInGame _returnvalue true))
    (:then_1
      (Rendering|SetActorHiddenInGame false))
    (:then_2
      (Rendering|SetActorHiddenInGame false)
      (Rendering|SetActorHiddenInGame false)
      (Rendering|SetActorHiddenInGame false))))

(event EventBeginPlay
  (Utilities|FlowControl|Sequence
    (:then_1
      (bind _asuxt_pressable_button_actor (Utilities|Casting|CastToUxtPressableButtonActor (Variables|/Script/Engine.ChildActorComponent|GetChildActor (Variables|Actor|GetCloseButton))))
      (EventDispatchers|BindEventtoOnButtonReleased (Variables|/Script/UXTools.UxtBasePressableButtonActor|GetButtonComponent _asuxt_pressable_button_actor) (delegate Custom|Close)))))

(fn ConstructionScript
  (bind _showexperimentalwarning (Variables|DescriptionPanel|GetShowExperimentalWarning))
  (Rendering|SetVisibility (Variables|Default|GetWarningBodyText) _showexperimentalwarning false)
  (Rendering|SetVisibility (Variables|Default|GetWarningTitleText) _showexperimentalwarning false))

(fn CloseParent)