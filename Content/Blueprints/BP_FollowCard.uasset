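; Mixed reality card panel with a UX Tools pin toggle, able to recenter the headset while keeping its placement relative to the user.
; Construction caches the pin button and toggle state from a child actor.
; RepositionLevel checks the pin, converts the panel's transform to a yaw-only, headset-relative one and applies it before resetting headset orientation and position, avoiding jitter.
; BeginPlay and Tick only call the parent.
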(event EventBeginPlay
  (|CallParentFunction))

(event EventTick
  (params (DeltaSeconds :type Float%20%28single-precision%29))
  (|CallParentFunction DeltaSeconds))

(event EventEndPlay
  (params (EndPlayReason :type EEndPlayReason%20Enum :default "Destroyed")))

(fn ConstructionScript
  (|CallParentFunction)
  (bind _asuxt_pressable_toggle_button_actor (Utilities|Casting|CastToUxtPressableToggleButtonActor (Variables|/Script/Engine.ChildActorComponent|GetChildActor (Variables|Default|GetButton_Pin))))
  (Variables|Default|SetPinButton (Variables|/Script/UXTools.UxtBasePressableButtonActor|GetButtonComponent _asuxt_pressable_toggle_button_actor))
  (Variables|Default|SetPinButtonState (Variables|/Script/UXTools.UxtPressableToggleButtonActor|GetToggleStateComponent _asuxt_pressable_toggle_button_actor)))

(fn RepositionLevel
  (Utilities|FlowControl|Sequence
    (:then_0
      ;[1 1 1] Pin panel before headset transform reset
      (Variables|/Script/UXTools.UxtToggleStateComponent|SetbIsChecked (Variables|Default|GetPinButtonState) true))
    (:then_1
      ;[1 1 1] Caching panel transform relative to headset
      (LocalVariables|SetRotationOffset (Class|KismetMathLibrary|NegateRotator (Math|Conversions|RotationFromXVector (Math|Vector|ProjectVectorontoPlane (Math|Vector|GetForwardVector (.DeviceRotation (Class|HeadMountedDisplayFunctionLibrary|GetOrientationandPosition))) "0, 0,1.000000")))))
    (:then_2
      (LocalVariables|SetLocationOffset (Math|Vector|RotateVector (- (Transformation|GetWorldLocation (Variables|Default|GetScene)) (.DevicePosition (Class|HeadMountedDisplayFunctionLibrary|GetOrientationandPosition))) (LocalVariables|GetRotationOffset))))
    (:then_3
      ;[1 1 1] Applying panel cached transform before headset reset to avoid jitter
      (Transformation|SetWorldLocation (Variables|Default|GetScene) (LocalVariables|GetLocationOffset) false false)
      (Transformation|SetWorldRotation (Variables|Default|GetScene) (Math|Rotator|CombineRotators (Transformation|GetWorldRotation (Variables|Default|GetScene)) (LocalVariables|GetRotationOffset)) false false))
    (:then_4
      (Class|HeadMountedDisplayFunctionLibrary|ResetOrientationandPosition 0.0 "OrientationAndPosition" :!pinned true) ; Reseting headset transform
    )))