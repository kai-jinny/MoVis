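; BP_QR is an actor that reacts to AR-tracked QR codes and places a model in the world.
; On each tracked geometry update, it draws a debug box and object name at a point derived from the code's transform and estimated size.
; It spawns BP_QRModel there only while BP_LevelDatabase's QRModelOn is false, then sets that flag to prevent repeat spawns.
; The image-added handler only casts, and the geometry-added handler is empty.
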(event OnAddTrackedImage(ARTrackableNotify)
  (params (TrackedImage :type AR%20Tracked%20Image%20Object%20Reference))
  (bind _asartracked_qrcode (Utilities|Casting|CastToARTrackedQRCode TrackedImage)))

(event OnUpdateTrackedGeometry(ARTrackableNotify)
  (params (TrackedGeometry :type AR%20Tracked%20Geometry%20Object%20Reference))
  (bind _asartracked_qrcode (Utilities|Casting|CastToARTrackedQRCode TrackedGeometry))
  (Rendering|Debug|DrawDebugString (Math|Transform|TransformLocation (Class|ARTrackedGeometry|GetLocaltoWorldTransform _asartracked_qrcode) (/ (Math|Vector|MakeVector 0.3 (.X (Math|Vector2D|BreakVector2D (Class|ARTrackedImage|GetEstimateSize _asartracked_qrcode))) (.Y (Math|Vector2D|BreakVector2D (Class|ARTrackedImage|GetEstimateSize _asartracked_qrcode)))) 2.0)) (Utilities|GetDisplayName _asartracked_qrcode) 0 "(R=1.000000,G=1.000000,B=1.000000,A=1.000000)")
  (Rendering|Debug|DrawDebugBox (Math|Transform|TransformLocation (Class|ARTrackedGeometry|GetLocaltoWorldTransform _asartracked_qrcode) (/ (Math|Vector|MakeVector 0.3 (.X (Math|Vector2D|BreakVector2D (Class|ARTrackedImage|GetEstimateSize _asartracked_qrcode))) (.Y (Math|Vector2D|BreakVector2D (Class|ARTrackedImage|GetEstimateSize _asartracked_qrcode)))) 2.0)) (/ (Math|Vector|MakeVector 0.3 (.X (Math|Vector2D|BreakVector2D (Class|ARTrackedImage|GetEstimateSize _asartracked_qrcode))) (.Y (Math|Vector2D|BreakVector2D (Class|ARTrackedImage|GetEstimateSize _asartracked_qrcode)))) 2.0) "(R=1.000000,G=0.046394,B=0.000000,A=1.000000)" (Math|Transform|TransformRotation (Class|ARTrackedGeometry|GetLocaltoWorldTransform _asartracked_qrcode) "0, 0, 0") 1.0 1.0)
  (bind _returnvalue (Actor|GetActorOfClass "/Game/Blueprints/BP_LevelDatabase.BP_LevelDatabase_C"))
  (if (Math|Boolean|Equal(Boolean) false (Variables|/Game/Blueprints/BP_LevelDatabase.BP_LevelDatabase_C|GetQRModelOn _returnvalue))
    (Game|SpawnActorfromClass "/Game/Blueprints/BP_QRModel.BP_QRModel_C" (Math|Conversions|ToTransform(Vector) (Math|Transform|TransformLocation (Class|ARTrackedGeometry|GetLocaltoWorldTransform _asartracked_qrcode) (/ (Math|Vector|MakeVector 0.3 (.X (Math|Vector2D|BreakVector2D (Class|ARTrackedImage|GetEstimateSize _asartracked_qrcode))) (.Y (Math|Vector2D|BreakVector2D (Class|ARTrackedImage|GetEstimateSize _asartracked_qrcode)))) 2.0))) "Undefined" 0 0)
    (Variables|/Game/Blueprints/BP_LevelDatabase.BP_LevelDatabase_C|SetQRModelOn _returnvalue true)))

(event OnAddTrackedGeometry(ARTrackableNotify)
  (params (TrackedGeometry :type AR%20Tracked%20Geometry%20Object%20Reference)))

(event EventBeginPlay)

(event Collision|EventActorBeginOverlap
  (params (OtherActor :type Actor%20Object%20Reference)))

(event EventTick
  (params (DeltaSeconds :type Float%20%28single-precision%29)))

(fn ConstructionScript)