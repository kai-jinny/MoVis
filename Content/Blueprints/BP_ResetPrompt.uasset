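; BP_ResetPrompt is a mixed reality confirmation prompt with Yes and No UXT pressable buttons for resetting the scene.
; On BeginPlay it hides the prompt actor, found by class lookup, and binds both child-actor buttons' release events.
; Yes reloads through the Loader_Auto1 level after a short delay, only if BP_LevelDatabase's ResetPromptOpen flag is set.
; No hides the prompt and clears that flag.
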(event Custom|Close
  (params (Button :type Uxt%20Pressable%20Button%20Component%20Object%20Reference) (Pointer :type Uxt%20Pointer%20Component%20Object%20Reference))
  (bind _returnvalue (Actor|GetActorOfClass "BP_ResetPrompt_C"))
  (Rendering|SetActorHiddenInGame _returnvalue true)
  (bind _outactors (Actor|GetAllActorsOfClass "/Game/Blueprints/BP_LevelDatabase.BP_LevelDatabase_C"))
  (Variables|/Game/Blueprints/BP_LevelDatabase.BP_LevelDatabase_C|SetResetPromptOpen (Utilities|Array|Get(acopy) _outactors) false))

(event Custom|Reset%20Scene
  (params (Button :type Uxt%20Pressable%20Button%20Component%20Object%20Reference) (Pointer :type Uxt%20Pointer%20Component%20Object%20Reference))
  (bind _outactors (Actor|GetAllActorsOfClass "/Game/Blueprints/BP_LevelDatabase.BP_LevelDatabase_C"))
  (if (Variables|/Game/Blueprints/BP_LevelDatabase.BP_LevelDatabase_C|GetResetPromptOpen (Utilities|Array|Get(acopy) _outactors))
    (Utilities|FlowControl|Delay 0.25)
    (Game|OpenLevel(byName) "Loader_Auto1")))

(event EventBeginPlay
  (bind _returnvalue (Actor|GetActorOfClass "BP_ResetPrompt_C"))
  (Rendering|SetActorHiddenInGame _returnvalue true)
  (Utilities|FlowControl|Sequence
    (:then_0
      (bind _asuxt_base_pressable_button_actor (Utilities|Casting|CastToUxtBasePressableButtonActor (Variables|/Script/Engine.ChildActorComponent|GetChildActor (Variables|Default|GetYesButton))))
      (EventDispatchers|BindEventtoOnButtonReleased (Variables|/Script/UXTools.UxtBasePressableButtonActor|GetButtonComponent _asuxt_base_pressable_button_actor) (delegate Custom|Reset%20Scene)))
    (:then_1
      (bind _asuxt_pressable_button_actor (Utilities|Casting|CastToUxtPressableButtonActor (Variables|/Script/Engine.ChildActorComponent|GetChildActor (Variables|Default|GetNoButton))))
      (EventDispatchers|BindEventtoOnButtonReleased (Variables|/Script/UXTools.UxtBasePressableButtonActor|GetButtonComponent _asuxt_pressable_button_actor) (delegate Custom|Close)))))

(fn ConstructionScript)

(fn CloseParent)