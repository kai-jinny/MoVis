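; Palm-up hand menu for an AR molecule viewer, built on UXT pressable buttons bound at BeginPlay.
; Previous/Next cycle three protein models through BP_LevelDatabase, swapping BP_Model meshes, materials and BP_FollowCard labels.
; Other buttons adjust light intensity, reset the model's transform, open the scene reset prompt and run STAT FPS.
; A QR tracking toggle exists, but its button binding is disconnected.
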(event OnConstraintActivated(UxtPalmUpConstraint)
  (Class|UxtUIElementComponent|SetUIVisibility (Variables|Default|GetUxtUIElement) "Show"))

(event OnConstraintDeactivated(UxtPalmUpConstraint)
  (Class|UxtUIElementComponent|SetUIVisibility (Variables|Default|GetUxtUIElement) "Hide"))

(event Custom|Show%20FPS
  (params (Button :type Uxt%20Pressable%20Button%20Component%20Object%20Reference) (Pointer :type Uxt%20Pointer%20Component%20Object%20Reference))
  (Development|ExecuteConsoleCommand "STAT FPS" 0))

(event Custom|Previous%20Model
  (params (Button :type Uxt%20Pressable%20Button%20Component%20Object%20Reference) (Pointer :type Uxt%20Pointer%20Component%20Object%20Reference))
  ;[1 1 1] Previous Model
  (bind _returnvalue (Actor|GetActorOfClass "/Game/Blueprints/BP_Model.BP_Model_C"))
  (bind _returnvalue_2 (Actor|GetActorOfClass "/Game/Blueprints/BP_LevelDatabase.BP_LevelDatabase_C"))
  (bind _returnvalue_3 (Actor|GetActorOfClass "/Game/Blueprints/BP_LevelDatabase.BP_LevelDatabase_C"))
  (if (<= (Variables|/Game/Blueprints/BP_LevelDatabase.BP_LevelDatabase_C|GetCurrentModel _returnvalue_2) 0)
    (Variables|/Game/Blueprints/BP_LevelDatabase.BP_LevelDatabase_C|SetCurrentModel _returnvalue_3 2)
    (else
      (Math|Integer|DecrementInt (Variables|/Game/Blueprints/BP_LevelDatabase.BP_LevelDatabase_C|GetCurrentModel _returnvalue_2)
        (:%20%20
          _))))
  (bind _returnvalue_4 (Actor|GetActorOfClass "/Game/Blueprints/BP_LevelDatabase.BP_LevelDatabase_C"))
  (Components|StaticMesh|SetStaticMesh (Variables|/Game/Blueprints/BP_Model.BP_Model_C|GetMoleculeMesh _returnvalue) (Utilities|Select :Index (Variables|/Game/Blueprints/BP_LevelDatabase.BP_LevelDatabase_C|GetCurrentModel _returnvalue_4) :Option%200 "/Game/Assets/6lu7_outer.6lu7_outer" :Option%201 "/Game/Assets/petOuter.petOuter" :Option%202 "/Game/Assets/N3_outer.N3_outer"))
  (Rendering|Material|SetMaterial (Variables|/Game/Blueprints/BP_Model.BP_Model_C|GetMoleculeMesh _returnvalue) 0 (Utilities|Select :Index (Variables|/Game/Blueprints/BP_LevelDatabase.BP_LevelDatabase_C|GetCurrentModel _returnvalue_4) :Option%200 "/Game/Assets/6lu7_outer_m.6lu7_outer_m" :Option%201 "/Game/Assets/m_petaseOuter.m_petaseOuter" :Option%202 "/Game/Assets/6lu7_outer_m.6lu7_outer_m"))
  (Components|StaticMesh|SetStaticMesh (Variables|/Game/Blueprints/BP_Model.BP_Model_C|GetMoleculeMesh2 _returnvalue) (Utilities|Select :Index (Variables|/Game/Blueprints/BP_LevelDatabase.BP_LevelDatabase_C|GetCurrentModel _returnvalue_4) :Option%200 "/Game/Assets/6lu7_inner.6lu7_inner" :Option%201 "/Game/Assets/petInner.petInner" :Option%202 "/Game/Assets/N3_inner.N3_inner"))
  (Rendering|Material|SetMaterial (Variables|/Game/Blueprints/BP_Model.BP_Model_C|GetMoleculeMesh2 _returnvalue) 0 (Utilities|Select :Index (Variables|/Game/Blueprints/BP_LevelDatabase.BP_LevelDatabase_C|GetCurrentModel _returnvalue_4) :Option%200 "/Game/Assets/6lu7_inner_m.6lu7_inner_m" :Option%201 "/Game/Assets/m_petaseInner.m_petaseInner" :Option%202 "/Game/Assets/m_N3_inner.m_N3_inner"))
  (Components|StaticMesh|SetStaticMesh (Variables|/Game/Blueprints/BP_Model.BP_Model_C|GetMoleculeMesh3 _returnvalue) (Utilities|Select :Index (Variables|/Game/Blueprints/BP_LevelDatabase.BP_LevelDatabase_C|GetCurrentModel _returnvalue_4) :Option%200 0 :Option%201 0 :Option%202 "/Game/Assets/ballStick_vmd_mol0_rep3.ballStick_vmd_mol0_rep3"))
  (Rendering|Material|SetMaterial (Variables|/Game/Blueprints/BP_Model.BP_Model_C|GetMoleculeMesh3 _returnvalue) 0 (Utilities|Select :Index (Variables|/Game/Blueprints/BP_LevelDatabase.BP_LevelDatabase_C|GetCurrentModel _returnvalue_4) :Option%200 "/Game/Assets/6lu7_outer_m.6lu7_outer_m" :Option%201 "/Game/Assets/m_petaseOuter.m_petaseOuter" :Option%202 "/Game/Assets/6lu7_outer_m.6lu7_outer_m"))
  (Components|StaticMesh|SetStaticMesh (Variables|/Game/Blueprints/BP_Model.BP_Model_C|GetMoleculeMesh4 _returnvalue) (Utilities|Select :Index (Variables|/Game/Blueprints/BP_LevelDatabase.BP_LevelDatabase_C|GetCurrentModel _returnvalue_4) :Option%200 0 :Option%201 0 :Option%202 "/Game/Assets/ballStick_vmd_mol0_rep2.ballStick_vmd_mol0_rep2"))
  (Rendering|Material|SetMaterial (Variables|/Game/Blueprints/BP_Model.BP_Model_C|GetMoleculeMesh4 _returnvalue) 0 (Utilities|Select :Index (Variables|/Game/Blueprints/BP_LevelDatabase.BP_LevelDatabase_C|GetCurrentModel _returnvalue_4) :Option%200 0 :Option%201 0 :Option%202 0))
  ;[1 1 1] Set Label
  (bind _returnvalue_5 (Actor|GetActorOfClass "/Game/Blueprints/BP_LevelDatabase.BP_LevelDatabase_C"))
  (Utilities|FlowControl|Sequence
    (:then_0
      (if (== (Variables|/Game/Blueprints/BP_LevelDatabase.BP_LevelDatabase_C|GetCurrentModel _returnvalue_5) 0)
        (bind _returnvalue_6 (Actor|GetActorOfClass "/Game/Blueprints/BP_FollowCard.BP_FollowCard_C"))
        (Rendering|SetVisibility (Variables|/Game/Blueprints/BP_FollowCard.BP_FollowCard_C|GetModelNameProtease _returnvalue_6) true false)
        (Rendering|SetVisibility (Variables|/Game/Blueprints/BP_FollowCard.BP_FollowCard_C|GetModelNamePetase _returnvalue_6) false false)))
    (:then_1
      (if (== (Variables|/Game/Blueprints/BP_LevelDatabase.BP_LevelDatabase_C|GetCurrentModel _returnvalue_5) 1)
        (bind _returnvalue_7 (Actor|GetActorOfClass "/Game/Blueprints/BP_FollowCard.BP_FollowCard_C"))
        (Rendering|SetVisibility (Variables|/Game/Blueprints/BP_FollowCard.BP_FollowCard_C|GetModelNameProtease _returnvalue_7) false false)
        (Rendering|SetVisibility (Variables|/Game/Blueprints/BP_FollowCard.BP_FollowCard_C|GetModelNamePetase _returnvalue_7) true false)))
    (:then_2
      (if (== (Variables|/Game/Blueprints/BP_LevelDatabase.BP_LevelDatabase_C|GetCurrentModel _returnvalue_5) 2)
        (bind _returnvalue_8 (Actor|GetActorOfClass "/Game/Blueprints/BP_FollowCard.BP_FollowCard_C"))
        (Rendering|SetVisibility (Variables|/Game/Blueprints/BP_FollowCard.BP_FollowCard_C|GetModelNameProtease _returnvalue_8) true false)
        (Rendering|SetVisibility (Variables|/Game/Blueprints/BP_FollowCard.BP_FollowCard_C|GetModelNamePetase _returnvalue_8) false false)))))

(event Custom|Next%20Model
  (params (Button :type Uxt%20Pressable%20Button%20Component%20Object%20Reference) (Pointer :type Uxt%20Pointer%20Component%20Object%20Reference))
  ;[1 1 1] Next Model
  (bind _returnvalue (Actor|GetActorOfClass "/Game/Blueprints/BP_Model.BP_Model_C"))
  (bind _returnvalue_2 (Actor|GetActorOfClass "/Game/Blueprints/BP_LevelDatabase.BP_LevelDatabase_C"))
  (bind _returnvalue_3 (Actor|GetActorOfClass "/Game/Blueprints/BP_LevelDatabase.BP_LevelDatabase_C"))
  (if (>= (Variables|/Game/Blueprints/BP_LevelDatabase.BP_LevelDatabase_C|GetCurrentModel _returnvalue_2) 2)
    (Variables|/Game/Blueprints/BP_LevelDatabase.BP_LevelDatabase_C|SetCurrentModel _returnvalue_3 0)
    (else
      (Math|Integer|IncrementInt (Variables|/Game/Blueprints/BP_LevelDatabase.BP_LevelDatabase_C|GetCurrentModel _returnvalue_2)
        (:%20%20
          _))))
  (bind _returnvalue_4 (Actor|GetActorOfClass "/Game/Blueprints/BP_LevelDatabase.BP_LevelDatabase_C"))
  (Components|StaticMesh|SetStaticMesh (Variables|/Game/Blueprints/BP_Model.BP_Model_C|GetMoleculeMesh _returnvalue) (Utilities|Select :Index (Variables|/Game/Blueprints/BP_LevelDatabase.BP_LevelDatabase_C|GetCurrentModel _returnvalue_4) :Option%200 "/Game/Assets/6lu7_outer.6lu7_outer" :Option%201 "/Game/Assets/petOuter.petOuter" :Option%202 "/Game/Assets/N3_outer.N3_outer"))
  (Rendering|Material|SetMaterial (Variables|/Game/Blueprints/BP_Model.BP_Model_C|GetMoleculeMesh _returnvalue) 0 (Utilities|Select :Index (Variables|/Game/Blueprints/BP_LevelDatabase.BP_LevelDatabase_C|GetCurrentModel _returnvalue_4) :Option%200 "/Game/Assets/6lu7_outer_m.6lu7_outer_m" :Option%201 "/Game/Assets/m_petaseOuter.m_petaseOuter" :Option%202 "/Game/Assets/6lu7_outer_m.6lu7_outer_m"))
  (Components|StaticMesh|SetStaticMesh (Variables|/Game/Blueprints/BP_Model.BP_Model_C|GetMoleculeMesh2 _returnvalue) (Utilities|Select :Index (Variables|/Game/Blueprints/BP_LevelDatabase.BP_LevelDatabase_C|GetCurrentModel _returnvalue_4) :Option%200 "/Game/Assets/6lu7_inner.6lu7_inner" :Option%201 "/Game/Assets/petInner.petInner" :Option%202 "/Game/Assets/N3_inner.N3_inner"))
  (Rendering|Material|SetMaterial (Variables|/Game/Blueprints/BP_Model.BP_Model_C|GetMoleculeMesh2 _returnvalue) 0 (Utilities|Select :Index (Variables|/Game/Blueprints/BP_LevelDatabase.BP_LevelDatabase_C|GetCurrentModel _returnvalue_4) :Option%200 "/Game/Assets/6lu7_inner_m.6lu7_inner_m" :Option%201 "/Game/Assets/m_petaseInner.m_petaseInner" :Option%202 "/Game/Assets/m_N3_inner.m_N3_inner"))
  (Components|StaticMesh|SetStaticMesh (Variables|/Game/Blueprints/BP_Model.BP_Model_C|GetMoleculeMesh3 _returnvalue) (Utilities|Select :Index (Variables|/Game/Blueprints/BP_LevelDatabase.BP_LevelDatabase_C|GetCurrentModel _returnvalue_4) :Option%200 0 :Option%201 0 :Option%202 "/Game/Assets/ballStick_vmd_mol0_rep3.ballStick_vmd_mol0_rep3"))
  (Rendering|Material|SetMaterial (Variables|/Game/Blueprints/BP_Model.BP_Model_C|GetMoleculeMesh3 _returnvalue) 0 (Utilities|Select :Index (Variables|/Game/Blueprints/BP_LevelDatabase.BP_LevelDatabase_C|GetCurrentModel _returnvalue_4) :Option%200 "/Game/Assets/6lu7_outer_m.6lu7_outer_m" :Option%201 "/Game/Assets/m_petaseOuter.m_petaseOuter" :Option%202 "/Game/Assets/6lu7_outer_m.6lu7_outer_m"))
  (Components|StaticMesh|SetStaticMesh (Variables|/Game/Blueprints/BP_Model.BP_Model_C|GetMoleculeMesh4 _returnvalue) (Utilities|Select :Index (Variables|/Game/Blueprints/BP_LevelDatabase.BP_LevelDatabase_C|GetCurrentModel _returnvalue_4) :Option%200 0 :Option%201 0 :Option%202 "/Game/Assets/ballStick_vmd_mol0_rep2.ballStick_vmd_mol0_rep2"))
  (Rendering|Material|SetMaterial (Variables|/Game/Blueprints/BP_Model.BP_Model_C|GetMoleculeMesh4 _returnvalue) 0 (Utilities|Select :Index (Variables|/Game/Blueprints/BP_LevelDatabase.BP_LevelDatabase_C|GetCurrentModel _returnvalue_4) :Option%200 0 :Option%201 0 :Option%202 0))
  ;[1 1 1] Set Label
  (bind _returnvalue_5 (Actor|GetActorOfClass "/Game/Blueprints/BP_LevelDatabase.BP_LevelDatabase_C"))
  (Utilities|FlowControl|Sequence
    (:then_0
      (if (== (Variables|/Game/Blueprints/BP_LevelDatabase.BP_LevelDatabase_C|GetCurrentModel _returnvalue_5) 0)
        (bind _returnvalue_6 (Actor|GetActorOfClass "/Game/Blueprints/BP_FollowCard.BP_FollowCard_C"))
        (Rendering|SetVisibility (Variables|/Game/Blueprints/BP_FollowCard.BP_FollowCard_C|GetModelNameProtease _returnvalue_6) true false)
        (Rendering|SetVisibility (Variables|/Game/Blueprints/BP_FollowCard.BP_FollowCard_C|GetModelNamePetase _returnvalue_6) false false)))
    (:then_1
      (if (== (Variables|/Game/Blueprints/BP_LevelDatabase.BP_LevelDatabase_C|GetCurrentModel _returnvalue_5) 1)
        (bind _returnvalue_7 (Actor|GetActorOfClass "/Game/Blueprints/BP_FollowCard.BP_FollowCard_C"))
        (Rendering|SetVisibility (Variables|/Game/Blueprints/BP_FollowCard.BP_FollowCard_C|GetModelNameProtease _returnvalue_7) false false)
        (Rendering|SetVisibility (Variables|/Game/Blueprints/BP_FollowCard.BP_FollowCard_C|GetModelNamePetase _returnvalue_7) true false)))
    (:then_2
      (if (== (Variables|/Game/Blueprints/BP_LevelDatabase.BP_LevelDatabase_C|GetCurrentModel _returnvalue_5) 2)
        (bind _returnvalue_8 (Actor|GetActorOfClass "/Game/Blueprints/BP_FollowCard.BP_FollowCard_C"))
        (Rendering|SetVisibility (Variables|/Game/Blueprints/BP_FollowCard.BP_FollowCard_C|GetModelNameProtease _returnvalue_8) true false)
        (Rendering|SetVisibility (Variables|/Game/Blueprints/BP_FollowCard.BP_FollowCard_C|GetModelNamePetase _returnvalue_8) false false)))))

(event Custom|Reset%20Model
  (params (Button :type Uxt%20Pressable%20Button%20Component%20Object%20Reference) (Pointer :type Uxt%20Pointer%20Component%20Object%20Reference))
  ;[1 1 1] Reset Model
  (bind _returnvalue (Actor|GetActorOfClass "/Game/Blueprints/BP_Model.BP_Model_C"))
  (Transformation|SetActorTransform _returnvalue (Math|Transform|MakeTransform (Transformation|GetActorLocation _returnvalue) "0, 0, 0" "1,1,1")))

(event Custom|Reset%20Scene
  (params (Button :type Uxt%20Pressable%20Button%20Component%20Object%20Reference) (Pointer :type Uxt%20Pointer%20Component%20Object%20Reference))
  ;[1 1 1] Reset Scene
  (Rendering|SetActorHiddenInGame (Variables|Default|GetResetPrompt) false)
  (bind _outactors (Actor|GetAllActorsOfClass "/Game/Blueprints/BP_LevelDatabase.BP_LevelDatabase_C"))
  (Variables|/Game/Blueprints/BP_LevelDatabase.BP_LevelDatabase_C|SetResetPromptOpen (Utilities|Array|Get(acopy) _outactors) true))

(event Custom|Brighter
  (params (Button :type Uxt%20Pressable%20Button%20Component%20Object%20Reference) (Pointer :type Uxt%20Pointer%20Component%20Object%20Reference))
  ;[1 1 1] Brighter
  (bind _result (Math|Float|IncrementFloat (Variables|/Script/GraphicsTools.GTDirectionalLightComponent|GetLightIntensity (Actor|GetComponentbyClass (Variables|Default|GetLightActor) "/Script/GraphicsTools.GTDirectionalLightComponent")))
    (:%20%20
      (Variables|/Script/GraphicsTools.GTDirectionalLightComponent|SetLightIntensity (Actor|GetComponentbyClass (Variables|Default|GetLightActor) "/Script/GraphicsTools.GTDirectionalLightComponent") _result))))

(event Custom|Start%20Tracking
  (params (Button :type Uxt%20Pressable%20Button%20Component%20Object%20Reference) (Pointer :type Uxt%20Pointer%20Component%20Object%20Reference))
  (bind _returnvalue (Actor|GetActorOfClass "/Game/Blueprints/BP_LevelDatabase.BP_LevelDatabase_C"))
  (if (Variables|/Game/Blueprints/BP_LevelDatabase.BP_LevelDatabase_C|GetTrackingModeOn _returnvalue)
    (Variables|/Game/Blueprints/BP_LevelDatabase.BP_LevelDatabase_C|SetTrackingModeOn _returnvalue false)
    (bind _returnvalue_2 (Actor|GetActorOfClass "/Game/Blueprints/BP_Model.BP_Model_C"))
    (Rendering|SetActorHiddenInGame _returnvalue_2 false)
    (Class|ARBlueprintLibrary|ToggleARCapture false "QRCode")
    (bind _outactors (Actor|GetAllActorsOfClass "/Game/Blueprints/BP_QRModel.BP_QRModel_C"))
    (Actor|DestroyActor _outactors)
    (Rendering|SetVisibility (Variables|/Game/Blueprints/BP_FollowCard.BP_FollowCard_C|GetModelNameQRModel (stale _returnvalue_8)) false false)
    ;[1 1 1] Set Label
    (bind _returnvalue_3 (Actor|GetActorOfClass "/Game/Blueprints/BP_LevelDatabase.BP_LevelDatabase_C"))
    (Utilities|FlowControl|Sequence
      (:then_0
        (if (== (Variables|/Game/Blueprints/BP_LevelDatabase.BP_LevelDatabase_C|GetCurrentModel _returnvalue_3) 0)
          (bind _returnvalue_4 (Actor|GetActorOfClass "/Game/Blueprints/BP_FollowCard.BP_FollowCard_C"))
          (Rendering|SetVisibility (Variables|/Game/Blueprints/BP_FollowCard.BP_FollowCard_C|GetModelNameProtease _returnvalue_4) true false)
          (Rendering|SetVisibility (Variables|/Game/Blueprints/BP_FollowCard.BP_FollowCard_C|GetModelNamePetase _returnvalue_4) false false)))
      (:then_1
        (if (== (Variables|/Game/Blueprints/BP_LevelDatabase.BP_LevelDatabase_C|GetCurrentModel _returnvalue_3) 1)
          (bind _returnvalue_5 (Actor|GetActorOfClass "/Game/Blueprints/BP_FollowCard.BP_FollowCard_C"))
          (Rendering|SetVisibility (Variables|/Game/Blueprints/BP_FollowCard.BP_FollowCard_C|GetModelNameProtease _returnvalue_5) false false)
          (Rendering|SetVisibility (Variables|/Game/Blueprints/BP_FollowCard.BP_FollowCard_C|GetModelNamePetase _returnvalue_5) true false)))
      (:then_2
        (if (== (Variables|/Game/Blueprints/BP_LevelDatabase.BP_LevelDatabase_C|GetCurrentModel _returnvalue_3) 2)
          (bind _returnvalue_6 (Actor|GetActorOfClass "/Game/Blueprints/BP_FollowCard.BP_FollowCard_C"))
          (Rendering|SetVisibility (Variables|/Game/Blueprints/BP_FollowCard.BP_FollowCard_C|GetModelNameProtease _returnvalue_6) true false)
          (Rendering|SetVisibility (Variables|/Game/Blueprints/BP_FollowCard.BP_FollowCard_C|GetModelNamePetase _returnvalue_6) false false))))
    (else
      (Variables|/Game/Blueprints/BP_LevelDatabase.BP_LevelDatabase_C|SetTrackingModeOn _returnvalue true)
      (bind _returnvalue_7 (Actor|GetActorOfClass "/Game/Blueprints/BP_Model.BP_Model_C"))
      (Rendering|SetActorHiddenInGame _returnvalue_7 true)
      (bind _returnvalue_8 (Actor|GetActorOfClass "/Game/Blueprints/BP_FollowCard.BP_FollowCard_C"))
      (Rendering|SetVisibility (Variables|/Game/Blueprints/BP_FollowCard.BP_FollowCard_C|GetModelNamePetase _returnvalue_8) false false)
      (Rendering|SetVisibility (Variables|/Game/Blueprints/BP_FollowCard.BP_FollowCard_C|GetModelNameQRModel _returnvalue_8) true false)
      (Class|ARBlueprintLibrary|ToggleARCapture true "QRCode")
      (bind _outactors_2 (Actor|GetAllActorsOfClass "/Game/Blueprints/BP_QRModel.BP_QRModel_C"))
      (Development|PrintString (Utilities|String|ToString(Integer) (Utilities|Array|Length _outactors_2))))))

(event Custom|Dimmer
  (params (Button :type Uxt%20Pressable%20Button%20Component%20Object%20Reference) (Pointer :type Uxt%20Pointer%20Component%20Object%20Reference))
  ;[1 1 1] Dimmer
  (bind _result (Math|Float|DecrementFloat (Variables|/Script/GraphicsTools.GTDirectionalLightComponent|GetLightIntensity (Actor|GetComponentbyClass (Variables|Default|GetLightActor) "/Script/GraphicsTools.GTDirectionalLightComponent")))
    (:%20%20
      (Variables|/Script/GraphicsTools.GTDirectionalLightComponent|SetLightIntensity (Actor|GetComponentbyClass (Variables|Default|GetLightActor) "/Script/GraphicsTools.GTDirectionalLightComponent") _result))))

(event EventBeginPlay
  (|CallParentFunction)
  (Utilities|FlowControl|Sequence
    (:then_0
      ;[1 1 1] Previous Model
      (bind _asuxt_pressable_button_actor (Utilities|Casting|CastToUxtPressableButtonActor (Variables|/Script/Engine.ChildActorComponent|GetChildActor (Variables|Default|GetButton%201))))
      (EventDispatchers|BindEventtoOnButtonReleased (Variables|/Script/UXTools.UxtBasePressableButtonActor|GetButtonComponent _asuxt_pressable_button_actor) (delegate Custom|Previous%20Model)))
    (:then_1
      ;[1 1 1] Next Model
      (bind _asuxt_pressable_button_actor_2 (Utilities|Casting|CastToUxtPressableButtonActor (Variables|/Script/Engine.ChildActorComponent|GetChildActor (Variables|Default|GetButton%202))))
      (EventDispatchers|BindEventtoOnButtonReleased (Variables|/Script/UXTools.UxtBasePressableButtonActor|GetButtonComponent _asuxt_pressable_button_actor_2) (delegate Custom|Next%20Model)))
    (:then_2
      ;[1 1 1] Dimmer
      (bind _asuxt_pressable_button_actor_3 (Utilities|Casting|CastToUxtPressableButtonActor (Variables|/Script/Engine.ChildActorComponent|GetChildActor (Variables|Default|GetButton%203))))
      (EventDispatchers|BindEventtoOnButtonReleased (Variables|/Script/UXTools.UxtBasePressableButtonActor|GetButtonComponent _asuxt_pressable_button_actor_3) (delegate Custom|Dimmer)))
    (:then_3
      ;[1 1 1] Brighter
      (bind _asuxt_pressable_button_actor_4 (Utilities|Casting|CastToUxtPressableButtonActor (Variables|/Script/Engine.ChildActorComponent|GetChildActor (Variables|Default|GetButton%204))))
      (EventDispatchers|BindEventtoOnButtonReleased (Variables|/Script/UXTools.UxtBasePressableButtonActor|GetButtonComponent _asuxt_pressable_button_actor_4) (delegate Custom|Brighter)))
    (:then_4
      ;[1 1 1] Reset Model
      (bind _asuxt_pressable_button_actor_5 (Utilities|Casting|CastToUxtPressableButtonActor (Variables|/Script/Engine.ChildActorComponent|GetChildActor (Variables|Default|GetButton%205))))
      (EventDispatchers|BindEventtoOnButtonReleased (Variables|/Script/UXTools.UxtBasePressableButtonActor|GetButtonComponent _asuxt_pressable_button_actor_5) (delegate Custom|Reset%20Model)))
    (:then_5
      ;[1 1 1] Reset Scene
      (bind _asuxt_pressable_button_actor_6 (Utilities|Casting|CastToUxtPressableButtonActor (Variables|/Script/Engine.ChildActorComponent|GetChildActor (Variables|Default|GetButton%206))))
      (EventDispatchers|BindEventtoOnButtonReleased (Variables|/Script/UXTools.UxtBasePressableButtonActor|GetButtonComponent _asuxt_pressable_button_actor_6) (delegate Custom|Reset%20Scene)))
    (:then_7
      (bind _asuxt_pressable_button_actor_7 (Utilities|Casting|CastToUxtPressableButtonActor (Variables|/Script/Engine.ChildActorComponent|GetChildActor (Variables|Default|GetButton%208))))
      (EventDispatchers|BindEventtoOnButtonReleased (Variables|/Script/UXTools.UxtBasePressableButtonActor|GetButtonComponent _asuxt_pressable_button_actor_7) (delegate Custom|Show%20FPS)))))

(fn ConstructionScript)